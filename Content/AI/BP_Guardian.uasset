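; BP_Guardian is an AI guardian character that exposes attack, patrol route and movement speed functions.
; Attack is a placeholder that prints a debug string and immediately calls the OnAttackEnd dispatcher, while the montage playback meant to signal completion is left disconnected.
; GetPatrolRoute returns the stored route, and SetMovementSpeed maps an idle-to-sprint speed enum onto the CharacterMovement max walk speed.
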(event Custom|Attack
  (Development|PrintString "PUTIASO")
  (Default|CallOnAttackEnd)
  (Default|CallOnAttackEnd))

(event EventBeginPlay)

(fn ConstructionScript)

(fn GetPatrolRoute
  (return (Variables|Default|GetPatrolRoute)))

(fn SetMovementSpeed
  (params (Speed :type E_MovementSpeed%20Enum :default "NewEnumerator0"))
  (bind _output_get (Variables|/Script/Engine.CharacterMovementComponent|SetMaxWalkSpeed (Variables|Character|GetCharacterMovement) (Utilities|Select :Index Speed :NewEnumerator0 0.0 :NewEnumerator1 133.3 :NewEnumerator2 266.6 :NewEnumerator3 4e+02)))
  (return _output_get))