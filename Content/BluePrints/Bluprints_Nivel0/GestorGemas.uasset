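; GestorGemas is a gem manager that sets up a level's collectible gems on BeginPlay.
; It loads or creates the GemaSaveSlot2 save and prints the saved gem record.
; It gathers PosicionGema-tagged locations, then spawns gems at random entries until GemasCreadas reaches four, removing a separately randomized index each time, so positions can repeat.
; Finally it tells Puerta to update its points and max score.
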(event Custom|ObtenerArrayPosiciones
  ;[0.15 0.15 0.15 0.5] Obtener array de posiciones
  (bind _outactors (Actor|GetAllActorswithTag "PosicionGema"))
  (for _array_element _outactors
    (Utilities|Array|Add (Variables|Default|GetWaypointsPosiciones) (Transformation|GetActorLocation _array_element))))

(event Custom|CrearGemasAleatorias
  (bind _waypointsposiciones (Variables|Default|GetWaypointsPosiciones))
  (bind (_outitem _outindex) (Utilities|Array|Random _waypointsposiciones))
  ;[0.15 0.15 0.15 0.5] Crear gemas en posiciones aleatorias v1
  (while (< (Variables|Default|GetGemasCreadas) 4)
    (Game|SpawnActorfromClass "/Game/BluePrints/Bluprints_Nivel0/GemaBlueprint.GemaBlueprint_C" (Math|Transform|MakeTransform _outitem) "Undefined" "MultiplyWithRoot" 0 0)
    (Utilities|Array|RemoveIndex _waypointsposiciones _outindex)
    (Variables|Default|SetGemasCreadas (+ (Variables|Default|GetGemasCreadas) 1))))

(event Custom|CargarGemasColeccionadas
  ;[0.15 0.15 0.15 0.5] Cargar Gemas guardadas - persistencia de datos
  (bind _returnvalue (SaveGame|DoesSaveGameExist "GemaSaveSlot2"))
  (if _returnvalue
    (bind _returnvalue_2 (SaveGame|LoadGamefromSlot "GemaSaveSlot2"))
    (bind _asgemas_save_game (Utilities|Casting|CastToGemas_SaveGame _returnvalue_2))
    (Development|PrintString (Utilities|String|Append "Max Gemas guardadas " (Utilities|String|ToString(Integer) (Variables|/Game/BluePrints/Bluprints_Nivel0/Gemas_SaveGame.Gemas_SaveGame_C|GetMaxGemasColeccionadas _asgemas_save_game))) true true "(R=0.000000,G=0.660000,B=1.000000,A=1.000000)" 5.0)
    (else
      (bind _returnvalue_3 (SaveGame|CreateSaveGameObject "/Game/BluePrints/Bluprints_Nivel0/Gemas_SaveGame.Gemas_SaveGame_C"))
      (bind _output_get (Variables|/Game/BluePrints/Bluprints_Nivel0/Gemas_SaveGame.Gemas_SaveGame_C|SetMaxGemasColeccionadas _returnvalue_3 0))
      (SaveGame|SaveGametoSlot _returnvalue_3 "GemaSaveSlot2")
      (Development|PrintString (Utilities|String|Append "Max gemas guardadas " (Utilities|String|ToString(Integer) _output_get)) true true "(R=0.000000,G=0.660000,B=1.000000,A=1.000000)" 5.0))))

(event EventBeginPlay
  (bind _puerta (Variables|Default|GetPuerta))
  ;[0.15 0.15 0.15 0.5] COMIENZO
  (CallFunction|CargarGemasColeccionadas)
  (CallFunction|ObtenerArrayPosiciones)
  (CallFunction|CrearGemasAleatorias)
  (Default|ActualizarPuntos _puerta)
  (Default|ActualizarScoreMax _puerta))

(event Collision|EventActorBeginOverlap
  (params (OtherActor :type Actor%20Object%20Reference)))

(event EventTick
  (params (DeltaSeconds :type Float%20%28single-precision%29)))

(fn ConstructionScript)