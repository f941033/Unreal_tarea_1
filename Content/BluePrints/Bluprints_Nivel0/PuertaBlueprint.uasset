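; Gem-locked door that opens when a Player-tagged actor touches its collision box with four spheres activated, only once because of a DoOnce.
; ActivarEsfera counts gems, lights a sphere, updates the HUD and saves any new record to a SaveGame slot.
; A timeline lowers the door mesh, restarting a five-second close timer each update.
; CerrarPuerta raises it with a second timeline, reverting sphere materials on each update.
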(event OnComponentBeginOverlap(BoxCollision)
  (params (OverlappedComponent :type Primitive%20Component%20Object%20Reference) (OtherActor :type Actor%20Object%20Reference) (OtherComp :type Primitive%20Component%20Object%20Reference) (OtherBodyIndex :type Integer) (bFromSweep :type Boolean) (SweepResult :type Hit%20Result%20Structure%20%28by%20ref%29))
  (if (Actor|ActorHasTag OtherActor "Player")
    (Development|PrintString "tocando puerta")
    (if (== (Variables|Default|GetContadorEsferaActivada) 4)
      (Utilities|FlowControl|DoOnce false
        (:Completed
          (Development|PrintString "abriendo puerta")
          (Audio|SpawnSoundatLocation "/Game/Assets/Nivel_0/Sonidos/puerta2.puerta2" (Transformation|GetActorLocation) "0, 0, 0" 1.0 1.0 0.0 0 0)
          (bind _newtrack_0 (Timeline|Timeline Play)
            (:Update
              (Transformation|SetRelativeLocation (Variables|Default|GetPuertaMesh) (Math|Vector|MakeVector 0.0 0.0 (Math|Float|Lerp 0.0 -3.8e+02 _newtrack_0)) false false)
              (Utilities|Time|SetTimerbyEvent (delegate Custom|CerrarPuerta) 5.0)))))
      (else
        (Development|PrintString (Utilities|String|ToString(Integer) (Variables|Default|GetContadorEsferaActivada)))))))

(event Custom|DesactivarEsfera
  ;[0.15 0.15 0.15 0.5] DESACTIVAR ESFERA
  (bind _output_get (Variables|Default|SetContadorEsferaActivada (+ (Variables|Default|GetContadorEsferaActivada) 1)))
  (switch int _output_get
    (:1
      (Rendering|Material|SetMaterial (Variables|Default|GetSphere1) 0 "/Game/Assets/Nivel_0/Materiales/mat_sphere_door.mat_sphere_door"))
    (:2
      (Rendering|Material|SetMaterial (Variables|Default|GetSphere2) 0 "/Game/Assets/Nivel_0/Materiales/mat_sphere_door.mat_sphere_door"))
    (:3
      (Rendering|Material|SetMaterial (Variables|Default|GetSphere3) 0 "/Game/Assets/Nivel_0/Materiales/mat_sphere_door.mat_sphere_door"))
    (:4
      (Rendering|Material|SetMaterial (Variables|Default|GetSphere4) 0 "/Game/Assets/Nivel_0/Materiales/mat_sphere_door.mat_sphere_door"))))

(event Custom|GuardarMaxGemas
  (bind _contadoresferaactivada (Variables|Default|GetContadorEsferaActivada))
  ;[0.15 0.15 0.15 0.5] Máximo número de Gemas guardadas - persistencia de datos
  (bind _returnvalue (SaveGame|LoadGamefromSlot "GemaSaveSlot2"))
  (bind _asgemas_save_game (Utilities|Casting|CastToGemas_SaveGame _returnvalue))
  (if (> _contadoresferaactivada (Variables|/Game/BluePrints/Bluprints_Nivel0/Gemas_SaveGame.Gemas_SaveGame_C|GetMaxGemasColeccionadas _asgemas_save_game))
    (bind _output_get (Variables|/Game/BluePrints/Bluprints_Nivel0/Gemas_SaveGame.Gemas_SaveGame_C|SetMaxGemasColeccionadas _asgemas_save_game _contadoresferaactivada))
    (SaveGame|SaveGametoSlot _asgemas_save_game "GemaSaveSlot2")
    (Development|PrintString (Utilities|String|Append "Max Gemas guardadas " (Utilities|String|ToString(Integer) _output_get)) true true "(R=0.000000,G=0.660000,B=1.000000,A=1.000000)" 1e+01)
    (CallFunction|ActualizarScoreMax)))

(event Custom|CerrarPuerta
  ;[0.15 0.15 0.15 0.5] Cerrar puerta
  (Audio|SpawnSoundatLocation "/Game/Assets/Nivel_0/Sonidos/puerta2.puerta2" (Transformation|GetActorLocation) "0, 0, 0" 1.0 1.0 0.0 0 0)
  (bind _newtrack_0 (Timeline|Timeline_0 Play)
    (:Update
      (Transformation|SetRelativeLocation (Variables|Default|GetPuertaMesh) (Math|Vector|MakeVector 0.0 0.0 (Math|Float|Lerp -3.8e+02 0.0 _newtrack_0)) false false)
      (Variables|Default|SetContadorEsferaActivada 0)
      (for _index (range 1 4)
        (CallFunction|DesactivarEsfera)))))

(event Custom|ActualizarScoreMax
  ;[0.15 0.15 0.15 0.5] Actualizar HUD con el máximo score guardado
  (bind _returnvalue (SaveGame|LoadGamefromSlot "GemaSaveSlot2"))
  (bind _asgemas_save_game (Utilities|Casting|CastToGemas_SaveGame _returnvalue))
  (bind _foundwidgets (Widget|GetAllWidgetsOfClass "/Game/Jorge/WB_PlayerUI.WB_PlayerUI_C" true))
  (Variables|/Game/Jorge/WB_PlayerUI.WB_PlayerUI_C|SetMaxScoreText (Utilities|Array|Get(acopy) _foundwidgets) (Utilities|Text|ToText(String) (Utilities|String|Append "Max Score: " (Utilities|String|ToString(Integer) (Variables|/Game/BluePrints/Bluprints_Nivel0/Gemas_SaveGame.Gemas_SaveGame_C|GetMaxGemasColeccionadas _asgemas_save_game))))))

(event Custom|ActivarEsfera
  ;[0.15 0.15 0.15 0.5] ACTIVAR ESFERA
  (bind _output_get (Variables|Default|SetContadorEsferaActivada (+ (Variables|Default|GetContadorEsferaActivada) 1)))
  (CallFunction|GuardarMaxGemas)
  (CallFunction|ActualizarPuntos)
  (if (== (Variables|Default|GetContadorEsferaActivada) 4)
    (Audio|SpawnSoundatLocation "/Game/Assets/Nivel_0/Sonidos/maxGemas.maxGemas" (Transformation|GetActorLocation) "0, 0, 0" 1.0 1.0 0.0 0 0))
  (switch int _output_get
    (:1
      (Rendering|Material|SetMaterial (Variables|Default|GetSphere1) 0 "/Game/Assets/Nivel_0/Materiales/mat_sphere_door_activated.mat_sphere_door_activated"))
    (:2
      (Rendering|Material|SetMaterial (Variables|Default|GetSphere2) 0 "/Game/Assets/Nivel_0/Materiales/mat_sphere_door_activated.mat_sphere_door_activated"))
    (:3
      (Rendering|Material|SetMaterial (Variables|Default|GetSphere3) 0 "/Game/Assets/Nivel_0/Materiales/mat_sphere_door_activated.mat_sphere_door_activated"))
    (:4
      (Rendering|Material|SetMaterial (Variables|Default|GetSphere4) 0 "/Game/Assets/Nivel_0/Materiales/mat_sphere_door_activated.mat_sphere_door_activated"))))

(event Custom|ActualizarPuntos
  ;[0.15 0.15 0.15 0.5] Actualizar HUD con gemas coleccionadas
  (bind _foundwidgets (Widget|GetAllWidgetsOfClass "/Game/Jorge/WB_PlayerUI.WB_PlayerUI_C" true))
  (Variables|/Game/Jorge/WB_PlayerUI.WB_PlayerUI_C|SetGemasText (Utilities|Array|Get(acopy) _foundwidgets) (Utilities|Text|ToText(String) (Utilities|String|Append (Utilities|String|Append "Gemas: " (Utilities|String|ToString(Integer) (Variables|Default|GetContadorEsferaActivada))) "/4"))))

(event EventBeginPlay
  (CallFunction|ActualizarPuntos)
  (CallFunction|ActualizarScoreMax))

(event Collision|EventActorBeginOverlap
  (params (OtherActor :type Actor%20Object%20Reference)))

(event EventTick
  (params (DeltaSeconds :type Float%20%28single-precision%29)))

(fn ConstructionScript)