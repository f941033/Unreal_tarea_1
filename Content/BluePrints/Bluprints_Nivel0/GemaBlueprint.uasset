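; GemaBlueprint is a collectible gem that spins slowly around its yaw axis each tick.
; When an actor tagged Player overlaps its sphere, it finds the first PuertaBlueprint in the level and calls ActivarEsfera on it.
; It then plays a powerup sound at its location and destroys itself, after printing a debug pickup message.
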(event OnComponentBeginOverlap(Sphere)
  (params (OverlappedComponent :type Primitive%20Component%20Object%20Reference) (OtherActor :type Actor%20Object%20Reference) (OtherComp :type Primitive%20Component%20Object%20Reference) (OtherBodyIndex :type Integer) (bFromSweep :type Boolean) (SweepResult :type Hit%20Result%20Structure%20%28by%20ref%29))
  (if (Actor|ActorHasTag OtherActor "Player")
    (Development|PrintString "Gema coleccionada")
    (bind _outactors (Actor|GetAllActorsOfClass "/Game/BluePrints/Bluprints_Nivel0/PuertaBlueprint.PuertaBlueprint_C"))
    (Default|ActivarEsfera (Utilities|Array|Get(acopy) _outactors))
    (Audio|SpawnSoundatLocation "/Game/Assets/Nivel_0/Sonidos/power-up.power-up" (Transformation|GetActorLocation) "0, 0, 0" 1.0 1.0 0.0 0 0)
    (Actor|DestroyActor)))

(event EventBeginPlay)

(event Collision|EventActorBeginOverlap
  (params (OtherActor :type Actor%20Object%20Reference)))

(event EventTick
  (params (DeltaSeconds :type Float%20%28single-precision%29))
  (Transformation|AddLocalRotation (Variables|Default|GetDefaultSceneRoot) (Math|Rotator|MakeRotator 0.0 0.0 (* DeltaSeconds 15.0)) false false))

(fn ConstructionScript)